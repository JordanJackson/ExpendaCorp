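; BP_Player_Overview is the overview camera pawn the player controls, panning across the world with Enhanced Input movement.
; On possession it registers itself with BP_PlayerController and spawns a BP_TestPlayerFPS at the origin if no FPS character exists, handing that reference to the controller.
; Each tick it traces Pawn objects under the cursor, prints the hit actor's name and sends it a highlight message.
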(event Input|EnhancedActionEvents|EnhancedInputActionIA_Move
  (params (ActionValue :type Vector%202D%20Structure) (ElapsedSeconds :type Float%20%28double-precision%29) (TriggeredSeconds :type Float%20%28double-precision%29) (InputAction :type Input%20Action%20Object%20Reference :default "/Game/ExpendaCorp/Input/IA_Move.IA_Move"))
  (Transformation|SetActorLocation (+ (Transformation|GetActorLocation) (* (Math|Vector|Normalize (+ (* (.x ActionValue) (Class|KismetMathLibrary|VectorRight)) (* (.y ActionValue) (Class|KismetMathLibrary|VectorForward)))) (Variables|Default|GetCameraMoveSpeed) (Utilities|Time|GetWorldDeltaSeconds))) false false))

(event EventTick
  (params (DeltaSeconds :type Float%20%28single-precision%29))
  (bind _ec_playercontroller (Variables|Default|GetEC_PlayerController)
    (:then
      (if (.ReturnValue (Class|PlayerController|GetHitResultUnderCursorforObjects _ec_playercontroller (Utilities|Array|MakeArray "ObjectTypeQuery3") true))
        (Development|PrintString (Utilities|GetDisplayName (.HitActor (Collision|BreakHitResult (.HitResult (Class|PlayerController|GetHitResultUnderCursorforObjects _ec_playercontroller (Utilities|Array|MakeArray "ObjectTypeQuery3") true))))))
        (Class|UnitInterface|Highlight(Message) (.HitActor (Collision|BreakHitResult (.HitResult (Class|PlayerController|GetHitResultUnderCursorforObjects _ec_playercontroller (Utilities|Array|MakeArray "ObjectTypeQuery3") true)))))))
    (:else)))

(event EventPossessed
  (params (NewController :type Controller%20Object%20Reference))
  (bind _asbp_player_controller (Utilities|Casting|CastToBP_PlayerController NewController))
  (bind _output_get (Variables|Default|SetEC_PlayerController _asbp_player_controller))
  (Variables|/Script/ExpendaCorp.ECPlayerController|SetOverviewPawn _output_get self)
  (Utilities|IsValid (Variables|Default|GetFPSCharacter)
    (:Is%20Not%20Valid
      (bind _returnvalue (Game|SpawnActorfromClass "/Game/ExpendaCorp/Blueprints/BP_TestPlayerFPS.BP_TestPlayerFPS_C" (Math|Transform|MakeTransform "0, 0, 0") "Undefined" "MultiplyWithRoot" 0 0))
      (bind _output_get_2 (Variables|Default|SetFPSCharacter _returnvalue))
      (Variables|/Script/ExpendaCorp.ECPlayerController|SetFPSCharacter _output_get _output_get_2))))

(fn ConstructionScript)